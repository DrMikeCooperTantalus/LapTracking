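; Lap-timing logic for a user of ordered lap gates, tracking current, last and best lap times.
; EnterGate accepts only the expected gate index, advances it or wraps after the last gate, and returns whether it matched.
; Crossing gate 0 restarts the timer, records any completed lap and fires new-lap and best-lap dispatchers.
; Tick computes the running time from wall-clock time-of-day differences rather than accumulated delta time.
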(event EventBeginPlay)

(event EventTick
  (params (DeltaSeconds :type Float%20%28single-precision%29))
  ;[1 1 1] If we've started a lap, get the time since we started
  (if (Variables|Default|GetLapStarted)
    (Variables|Default|SetCurrentLapTime (- (TimeOfDay|GetTimeOfDay (Math|DateTime|Now) :!class /Script/Engine.KismetMathLibrary) (TimeOfDay|GetTimeOfDay (Variables|Default|GetLapStartTime) :!class /Script/Engine.KismetMathLibrary)))))

(fn EnterGate
  (params (Index :type Integer) (LastGate :type Boolean))
  (bind _returnvalue (Class|KismetMathLibrary|TimespanZeroValue))
  (bind _currentlaptime (Variables|Default|GetCurrentLapTime))
  ;[1 1 1] If we've passed through our next gate...
  (if (== Index (Variables|Default|GetNextGate))
    (Utilities|FlowControl|Sequence
      (:then_0
        ;[1 1 1] Add 1 to NextGate
        (Variables|Default|SetNextGate (+ (Variables|Default|GetNextGate) 1)))
      (:then_1
        ;[1 1 1] Set NextGate back to 0 if we've completed the last one
        (if LastGate
          (Variables|Default|SetNextGate 0)))
      (:then_2
        ;[1 1 1] If we've crossed the 0 gate: start lap tracking, set our last lap time to the current one and set it as best if appropriate
        (if (== Index 0)
          (Variables|Default|SetLapStartTime (Math|DateTime|Now))
          (Variables|Default|SetLapStarted true)
          (if (> _currentlaptime _returnvalue)
            (Variables|Default|SetLastLapTime _currentlaptime)
            (Default|CallOnNewLap)
            (if (or (< _currentlaptime (Variables|Default|GetBestLapTime)) (== _returnvalue (Variables|Default|GetBestLapTime)))
              (Variables|Default|SetBestLapTime _currentlaptime)
              (Default|CallOnBestLap)))))
      (:then_3
        (return true)))
    (else
      (return false))))